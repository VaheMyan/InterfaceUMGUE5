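; BP_ButtonManager keeps a registry of buttons and toggles the objects they control when a change-visibility event fires.
; It binds to that event on BeginPlay and unbinds all handlers on EndPlay.
; On each event it loops over the registered buttons, calling OffObjects on those that are on and OnObjects on the rest.
; AddButton and RemoveButton maintain the collection.
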(event `self.ReceiveEndPlay`
  (params (EndPlayReason :type "EEndPlayReason Enum" :default "Destroyed"))
  (clear `self.ChangeObjectsVisibility`))

(event `self.ReceiveBeginPlay`
  (add `self.ChangeObjectsVisibility` (delegate `ChangeVisibility`)))

(event `ChangeVisibility`
  (bind _result (`BlueprintSetLibrary.Set_ToArray` (`self.Buttons`)))
  (for _array_element _result
    (bind _ison (`/Game/InterfaceUMG/Blueprints/BPI_Switchable.IsOn` _array_element))
    (if _ison
      (`/Game/InterfaceUMG/Blueprints/BPI_Switchable.OffObjects` _array_element)
      (else
        (`/Game/InterfaceUMG/Blueprints/BPI_Switchable.OnObjects` _array_element)))))

(fn `AddButton`
  (params (NewButton :type "/Game/InterfaceUMG/Blueprints/BP_Button Object Reference"))
  (`BlueprintSetLibrary.Set_Add` (`self.Buttons`) NewButton))

(fn `RemoveButton`
  (params (Button :type "/Game/InterfaceUMG/Blueprints/BP_Button Object Reference"))
  (returns (IsSuccess :type Boolean))
  (bind _returnvalue (`BlueprintSetLibrary.Set_Remove` (`self.Buttons`) Button))
  (return _returnvalue))

(fn `UserConstructionScript`)