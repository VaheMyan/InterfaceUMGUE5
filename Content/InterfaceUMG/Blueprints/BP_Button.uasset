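; BP_Button is an overlap-triggered button actor that can show or hide a linked group of objects.
; On BeginPlay it finds the BP_ButtonManager, then adds itself on any actor overlap and removes itself when overlap ends.
; OnObjects and OffObjects toggle each linked object's Cube visibility and set the state returned by IsOn.
; That state updates inside the loop, so it stays unchanged when Objects is empty.
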(event `self.ReceiveBeginPlay`
  (bind _returnvalue (`GameplayStatics.GetActorOfClass` "/Game/InterfaceUMG/Blueprints/BP_ButtonManager.BP_ButtonManager_C"))
  (set `self.ButtonManager` _returnvalue))

(event `self.ReceiveActorBeginOverlap`
  (params (OtherActor :type "Actor Object Reference"))
  (`/Game/InterfaceUMG/Blueprints/BP_ButtonManager.AddButton` (`self.ButtonManager`) self))

(event `self.ReceiveActorEndOverlap`
  (params (OtherActor :type "Actor Object Reference"))
  (`/Game/InterfaceUMG/Blueprints/BP_ButtonManager.RemoveButton` (`self.ButtonManager`) self))

(event `/Game/InterfaceUMG/Blueprints/BPI_Switchable.OnObjects`
  (bind _result (`BlueprintSetLibrary.Set_ToArray` (`self.Objects`)))
  (for _array_element _result
    (`SceneComponent.SetVisibility` (`/Game/InterfaceUMG/Blueprints/BP_Object.Cube` _array_element) true false)
    (set `self.IsObjectsOn` true)))

(event `/Game/InterfaceUMG/Blueprints/BPI_Switchable.OffObjects`
  (bind _result (`BlueprintSetLibrary.Set_ToArray` (`self.Objects`)))
  (for _array_element _result
    (`SceneComponent.SetVisibility` (`/Game/InterfaceUMG/Blueprints/BP_Object.Cube` _array_element) false false)
    (set `self.IsObjectsOn` false)))

(fn `IsOn`
  (returns (IsOn :type Boolean))
  (return (`self.IsObjectsOn`)))

(fn `UserConstructionScript`)